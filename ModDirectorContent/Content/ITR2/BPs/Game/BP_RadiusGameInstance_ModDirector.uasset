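; Modded Radius game instance that acts as a mod director, loading and notifying mod content.
; After game start and level load, it polls for ModDataActors until their count settles or scanning times out.
; ScanAndSpawn gathers their actor and object class lists, spawns or constructs them and passes itself as a reference.
; It relays level-load and in-game menu events to mod instances, respawning missing mod actors after each level load.
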(event Custom|PrintToModLoader
  (params (Message :type String)))

(event Custom|On%20Game%20Start%20Event)

(event Custom|On%20Finish%20Level%20Load%20Event
  (bind _returnvalue (Subsystems|GetRadiusLevelSubsystem))
  (bind _returnvalue_2 (Class|RadiusLevelSubsystem|GetCurrentLevel _returnvalue))
  (bind _asradius_player_character (Utilities|Casting|CastToRadiusPlayerCharacter (Game|GetPlayerCharacter 0))
    (:then
      (bind _output_get (Variables|Default|SetAs%20Radius%20Player%20Character _asradius_player_character))
      (Utilities|IsValid _output_get
        (:Is%20Valid
          (CallFunction|PrinttoModLoader "Got Player Character 0"))
        (:Is%20Not%20Valid
          (CallFunction|PrinttoModLoader "Cast to Radius Player Character Failed" :!label _label))))
    (:CastFailed
      (goto _label)))
  (CallFunction|PrinttoModLoader "Modded Instance on finish level load")
  (for _array_element (Variables|Default|GetConstructed%20Object%20Array)
    (Class|BPIModDirector|OnFinishLevelLoad(Message) _array_element _returnvalue_2))
  (bind _output_spawned_actors (CallFunction|RespawnMDActors))
  (for _array_element_2 _output_spawned_actors
    (Class|BPIModDirector|OnFinishLevelLoad(Message) _array_element_2 _returnvalue_2)))

(event Custom|InGameMenuOpened%20Event
  (for _array_element (Variables|Default|GetSpawned%20Actor%20Array)
    (Class|BPIModDirector|InGameMenuOpened(Message) _array_element))
  (for _array_element_2 (Variables|Default|GetConstructed%20Object%20Array)
    (Class|BPIModDirector|InGameMenuOpened(Message) _array_element_2)))

(event Custom|OnIngameMenuClosed%20Event
  (for _array_element (Variables|Default|GetSpawned%20Actor%20Array)
    (Class|BPIModDirector|OnIngameMenuClosed(Message) _array_element))
  (for _array_element_2 (Variables|Default|GetConstructed%20Object%20Array)
    (Class|BPIModDirector|InGameMenuOpened(Message) _array_element_2)))

(event EventOnGameStart
  (bind _returnvalue (Subsystems|GetRadiusEventsSubsystem))
  (|CallParentFunction)
  (EventDispatchers|BindEventtoOnGameStart _returnvalue (delegate Custom|On%20Game%20Start%20Event))
  (EventDispatchers|BindEventtoOnFinishLoadLevel _returnvalue (delegate Custom|On%20Finish%20Level%20Load%20Event))
  (EventDispatchers|BindEventtoOnIngameMenuOpened _returnvalue (delegate Custom|InGameMenuOpened%20Event))
  (EventDispatchers|BindEventtoOnIngameMenuClosed _returnvalue (delegate Custom|OnIngameMenuClosed%20Event))
  (CallFunction|PrinttoModLoader "Modded Instance initialized, delaying for MDactors to spawn")
  (if (Class|RadiusGameInstanceInterface|IsLoadLevelFinished) :!label _label
    (CallFunction|PrinttoModLoader "Modded Instance: Game Finished loading, delaying for Mod Data actors to spawn")
    (if (Variables|Default|GetMod%20Data%20Actor%20Found) :!label _label_2
      (if (Variables|Default|GetCount%20Changed) :!label _label_3
        (Utilities|FlowControl|Sequence
          (:then_0
            (goto _label_4 Reset))
          (:then_1
            (CallFunction|PrinttoModLoader "Count Changed, Resetting")
            (bind _count (Utilities|DoNComplete 5 :!label _label_4)
              (:Exit
                (CallFunction|PrinttoModLoader (Utilities|String|Append "Scan Count:" (Utilities|String|ToString(Integer) _count)))
                (Utilities|FlowControl|Delay 1.0)
                (bind _outactors (Actor|GetAllActorsOfClass "/Game/Mods/ModDirector/ModDataActor.ModDataActor_C" :!label _label_5))
                (if (> (Utilities|Array|Length _outactors) (Variables|Default|GetMod%20Data%20Actor%20Count))
                  (Variables|Default|SetMod%20Data%20Actor%20Count (Utilities|Array|Length _outactors))
                  (if (Variables|Default|GetMod%20Data%20Actor%20Found)
                    _
                    (else
                      (Variables|Default|SetMod%20Data%20Actor%20Found true)))
                  (Variables|Default|SetCount%20Changed true)
                  (goto _label_3)
                  (elif (Variables|Default|GetMod%20Data%20Actor%20Found)
                    (Variables|Default|SetCount%20Changed false)
                    (goto _label_3)
                    (else
                      (Variables|Default|SetScan%20Count (+ (Variables|Default|GetScan%20Count) 1))
                      (goto _label_2)))))
              (:Complete
                (CallFunction|ScanandSpawn)))))
        (elif (not (== (Variables|Default|GetScan%20Count) 4))
          (goto _label_4)))
      (elif (not (> (Variables|Default|GetScan%20Count) 25))
        (CallFunction|PrinttoModLoader (Utilities|String|Append "Scan Count:" (Utilities|String|ToString(Integer) (Variables|Default|GetScan%20Count))))
        (Utilities|FlowControl|Delay 0.5)
        (goto _label_5)
        (else
          (CallFunction|PrinttoModLoader "Scan cycle complete, found no Mod Data Actors"))))
    (else
      (Utilities|FlowControl|Delay 0.2)
      (goto _label))))

(event EventInit
  (|CallParentFunction))

(fn RespawnMDActors
  (for _array_element (Variables|Default|GetLoaded%20Actors)
    (bind _outactors (Actor|GetAllActorsOfClass _array_element))
    (if (== (Utilities|Array|Length _outactors) 0)
      (CallFunction|PrinttoModLoader (Utilities|String|Append (Utilities|GetClassDisplayName _array_element) " Does not exist anymore, respawning"))
      (bind _returnvalue (Game|SpawnActorfromClass _array_element (Math|Transform|MakeTransform "0, 0, 0" "0, 0, 0" "1.000000,1.000000,1.000000") "AlwaysSpawn" "SelectDefaultAtRuntime" 0 0))
      (else
        (for _array_element_2 _outactors
          (Default|OnFinishLevelLoad _array_element_2 (Class|RadiusLevelSubsystem|GetCurrentLevel (Subsystems|GetRadiusLevelSubsystem)))))))
  (bind _result (Utilities|Set|Union (LocalVariables|GetLocalFoundSet) (LocalVariables|GetLocalSet)))
  (bind _result_2 (Utilities|Set|ToArray _result))
  (Variables|Default|SetSpawned%20Actor%20Array _result_2))

(fn ScanandSpawn
  (CallFunction|PrinttoModLoader "Modded instance beginning scan for mod actors")
  (bind _outactors (Actor|GetAllActorsOfClass "/Game/Mods/ModDirector/ModDataActor.ModDataActor_C"))
  (for _array_element _outactors
    (bind _output_get (Variables|Default|SetCurrent%20Mod%20Data%20Actor _array_element))
    (Utilities|Array|Add (Variables|Default|GetMod%20Data%20Actor%20Array) _output_get)
    (CallFunction|PrinttoModLoader (Utilities|String|Append "Found " (Variables|/Game/Mods/ModDirector/ModDataActor.ModDataActor_C|GetModName _output_get) " Version " (Utilities|String|ToString(Integer) (Variables|/Game/Mods/ModDirector/ModDataActor.ModDataActor_C|GetModVersion _output_get))))
    (CallFunction|PrinttoModLoader (Utilities|String|Append "By" (Variables|/Game/Mods/ModDirector/ModDataActor.ModDataActor_C|GetModAuthor _output_get)))
    (for _array_element_2 (Variables|/Game/Mods/ModDirector/ModDataActor.ModDataActor_C|GetModActorArray _output_get)
      (Utilities|Array|AddUnique (Variables|Default|GetLoaded%20Actors) _array_element_2))
    (for _array_element_3 (Variables|/Game/Mods/ModDirector/ModDataActor.ModDataActor_C|GetModObjectArray _output_get)
      (Utilities|Array|AddUnique (Variables|Default|GetLoaded%20Objects) _array_element_3)))
  (for _array_element_4 (Variables|Default|GetLoaded%20Actors)
    (bind _output_get_2 (Variables|Default|SetCurrentModActor _array_element_4))
    (bind _outactors_2 (Actor|GetAllActorsOfClass _output_get_2))
    (if (!= (Utilities|Array|Length _outactors_2) 0)
      (CallFunction|PrinttoModLoader (Utilities|String|Append (Utilities|GetClassDisplayName _output_get_2) " is already spawned!"))
      (elif (Utilities|IsValidClass _output_get_2)
        (CallFunction|PrinttoModLoader (Utilities|String|Append (Utilities|GetClassDisplayName _output_get_2) " Is Valid"))
        (bind _returnvalue (Game|SpawnActorfromClass (Variables|Default|GetCurrentModActor) (Math|Transform|MakeTransform "0, 0, 0" "0, 0, 0" "1.000000,1.000000,1.000000") "AlwaysSpawn" "SelectDefaultAtRuntime" 0 0))
        (Class|BPIModDirector|Send/ReceiveInstanceRef(Message) _returnvalue self)
        (Utilities|Array|Add (Variables|Default|GetSpawned%20Actor%20Array) _returnvalue)
        (else
          (CallFunction|PrinttoModLoader (Utilities|String|Append (Utilities|GetClassDisplayName _output_get_2) " not a valid class"))))))
  (for _array_element_5 (Variables|Default|GetLoaded%20Objects)
    (bind _output_get_3 (Variables|Default|SetCurrent%20Object _array_element_5))
    (bind _returnvalue_2 (Game|ConstructObjectfromClass _output_get_3))
    (CallFunction|PrinttoModLoader (Utilities|String|Append "Constructing " (Utilities|GetClassDisplayName _output_get_3)))
    (Class|BPIModDirector|Send/ReceiveInstanceRef(Message) _returnvalue_2 self)
    (Utilities|Array|Add (Variables|Default|GetConstructed%20Object%20Array) _returnvalue_2))
  (for _array_element_6 (Variables|Default|GetSpawned%20Actor%20Array)
    (Class|BPIModDirector|ModDirectorLoadFinished(Message) _array_element_6 true))
  (for _array_element_7 (Variables|Default|GetConstructed%20Object%20Array)
    (Class|BPIModDirector|ModDirectorLoadFinished(Message) _array_element_7 true))
  (CallFunction|PrinttoModLoader "Scan and Spawn Function complete"))