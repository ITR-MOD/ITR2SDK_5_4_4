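; Gameplay game mode for Radius (ITR2) that acts as a mod loader, spawning mod actors and relaying game events to them.
; Shortly after BeginPlay it scans ModDataActors, gathers classes into LoadedAssets and spawns any not already present.
; Radius event bindings forward level-load and in-game menu events to spawned actors, respawning missing ones on level load.
; PrintToModLoader and the game-start handler are empty stubs.
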(event Custom|On%20Game%20Start%20Event)

(event Custom|On%20Finish%20Level%20Load%20Event
  (for _array_element (Variables|Default|GetSpawned%20Actor%20Array)
    (CallFunction|RespawnMDActors)
    (Default|OnFinishLevelLoad _array_element (Class|RadiusLevelSubsystem|GetCurrentLevel (Subsystems|GetRadiusLevelSubsystem)))))

(event Custom|InGameMenuOpened%20Event
  (for _array_element (Variables|Default|GetSpawned%20Actor%20Array)
    (Default|InGameMenuOpened _array_element)))

(event Custom|OnIngameMenuClosed%20Event
  (for _array_element (Variables|Default|GetSpawned%20Actor%20Array)
    (Default|OnIngameMenuClosed _array_element)))

(event EventBeginPlay
  (bind _returnvalue (Subsystems|GetRadiusEventsSubsystem))
  (EventDispatchers|BindEventtoOnGameStart _returnvalue (delegate Custom|On%20Game%20Start%20Event))
  (EventDispatchers|BindEventtoOnFinishLoadLevel _returnvalue (delegate Custom|On%20Finish%20Level%20Load%20Event))
  (EventDispatchers|BindEventtoOnIngameMenuOpened _returnvalue (delegate Custom|InGameMenuOpened%20Event))
  (EventDispatchers|BindEventtoOnIngameMenuClosed _returnvalue (delegate Custom|OnIngameMenuClosed%20Event))
  (Utilities|FlowControl|Delay 2.2)
  (CallFunction|ScanandSpawnModactors))

(event EventTick
  (params (DeltaSeconds :type Float%20%28single-precision%29)))

(fn ConstructionScript)

(fn ScanandSpawnModactors
  (bind _outactors (Actor|GetAllActorsOfClass "/Game/Mods/ModDirector/ModDataActor.ModDataActor_C"))
  (for _array_element _outactors
    (CallFunction|PrinttoModLoader (Utilities|String|Append "Found " (Variables|/Game/Mods/ModDirector/ModDataActor.ModDataActor_C|GetModName _array_element) "Version " (Utilities|String|ToString(Integer) (Variables|/Game/Mods/ModDirector/ModDataActor.ModDataActor_C|GetModVersion _array_element))))
    (CallFunction|PrinttoModLoader (Utilities|String|Append "By" (Variables|/Game/Mods/ModDirector/ModDataActor.ModDataActor_C|GetModAuthor _array_element)))
    (Utilities|Array|AddUnique (Variables|Default|GetLoaded%20Assets) 0))
  (for _array_element_2 (Variables|Default|GetLoaded%20Assets)
    (bind _output_get (Variables|Default|SetCurrentModActor _array_element_2))
    (bind _outactors_2 (Actor|GetAllActorsOfClass _output_get))
    (if (!= (Utilities|Array|Length _outactors_2) 0)
      (CallFunction|PrinttoModLoader (Utilities|String|Append (Utilities|GetClassDisplayName _output_get) " is already spawned!"))
      (elif (Utilities|IsValidClass _output_get)
        (CallFunction|PrinttoModLoader (Utilities|String|Append (Utilities|GetClassDisplayName _output_get) " Is Valid"))
        (bind _returnvalue (Game|SpawnActorfromClass (Variables|Default|GetCurrentModActor) (Math|Transform|MakeTransform "0, 0, 0" "0, 0, 0" "1.000000,1.000000,1.000000") "AlwaysSpawn" "SelectDefaultAtRuntime" 0 0))
        (Utilities|Array|Add (Variables|Default|GetSpawned%20Actor%20Array) _returnvalue)
        (else
          (CallFunction|PrinttoModLoader (Utilities|String|Append (Utilities|GetClassDisplayName _output_get) " not a valid class"))))))
  (CallFunction|PrinttoModLoader "Spawned All MDActors"))

(fn PrinttoModLoader
  (params (Message :type String)))

(fn RespawnMDActors
  (for _array_element (Variables|Default|GetLoaded%20Assets)
    (bind _outactors (Actor|GetAllActorsOfClass _array_element))
    (if (== (Utilities|Array|Length _outactors) 0)
      (CallFunction|PrinttoModLoader (Utilities|String|Append (Utilities|GetClassDisplayName _array_element) " Does not exist anymore, respawning"))
      (bind _returnvalue (Game|SpawnActorfromClass _array_element (Math|Transform|MakeTransform "0, 0, 0" "0, 0, 0" "1.000000,1.000000,1.000000") "AlwaysSpawn" "SelectDefaultAtRuntime" 0 0))
      (Utilities|Array|Add (Variables|Default|GetSpawned%20Actor%20Array) _returnvalue))))