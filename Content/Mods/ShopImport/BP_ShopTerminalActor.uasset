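; BP_ShopTerminalActor is a mod shop terminal that imports items from a master shop list and spawns them into a bin with an animated door.
; It passes the received list to its ShopImportSpawn widget, retrying until valid, and listens for that widget's import button.
; Import blocking-loads the item's soft class, spawns it at the child actor's transform as a shop item and opens the door.
; Removing the item closes the door after a delay and notifies the widget.
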(event OnComponentEndOverlap(Boxcollision)
  (params (OverlappedComponent :type Primitive%20Component%20Object%20Reference) (OtherActor :type Actor%20Object%20Reference) (OtherComp :type Primitive%20Component%20Object%20Reference) (OtherBodyIndex :type Integer))
  (bind _asradius_item_base (Utilities|Casting|CastToRadiusItemBase OtherActor))
  (if (== _asradius_item_base (Variables|Default|GetSpawned%20Item))
    (Utilities|FlowControl|Sequence
      (:then_0
        (Utilities|FlowControl|Delay 1.0)
        (bind _rotate_float (Timeline|Timeline ReverseFromEnd)
          (:Update
            (Transformation|SetRelativeRotation (Variables|Default|GetBinDoor) (Math|Rotator|MakeRotator (Math|Float|Lerp 0.0 -9e+01 _rotate_float) 0.0 0.0) false false))))
      (:then_1
        (Default|ItemRemovedfromBin (Variables|Default|GetAs%20Shop%20Import%20Spawn))))))

(event Custom|RotateDoorAndWait
  (bind _rotate_float (Timeline|Timeline Play)
    (:Update
      (Transformation|SetRelativeRotation (Variables|Default|GetBinDoor) (Math|Rotator|MakeRotator (Math|Float|Lerp 0.0 -9e+01 _rotate_float) 0.0 0.0) false false))))

(event Custom|ImportButtonPressed
  (params (TargetMap :type Map%20of%20Gameplay%20Tag%20Structures%20to%20Structs) (Key :type Gameplay%20Tag%20Structure%20%28by%20ref%29))
  (bind _spawngood (CallFunction|SpawnIteminBin (.Value (Utilities|Map|Find TargetMap Key))))
  (if _spawngood
    (Default|SetWIndexImport (Variables|Default|GetAs%20Shop%20Import%20Spawn))
    (else
      (CallFunction|PrinttoModLoader "ItemSpawnBad"))))

(event EventBeginPlay
  (bind _asshop_import_spawn (Utilities|Casting|CastToShopImportSpawn (UserInterface|GetUserWidgetObject (Variables|Default|GetRadiusWidget)))
    (:then
      (bind _output_get (Variables|Default|SetAs%20Shop%20Import%20Spawn _asshop_import_spawn))
      (EventDispatchers|BindEventtoImportButtonPressedEventDisp _output_get (delegate Custom|ImportButtonPressed))
      (Variables|Default|SetSpawnTransform (Transformation|GetWorldTransform (Variables|Default|GetChildActor))))
    (:CastFailed
      (CallFunction|PrinttoModLoader "Cast to Shop Import Spawn Failed"))))

(event Collision|EventActorBeginOverlap
  (params (OtherActor :type Actor%20Object%20Reference)))

(event EventTick
  (params (DeltaSeconds :type Float%20%28single-precision%29)))

(event EventSendMasterShopList
  (params (MasterShopList :type Map%20of%20Gameplay%20Tag%20Structures%20to%20Structs) (AdditionalCategories :type Map%20of%20Gameplay%20Tag%20Structures%20to%20Strings))
  (bind _as_shop_import_spawn (Variables|Default|GetAs%20Shop%20Import%20Spawn))
  (bind _output_get (Variables|Default|SetMaster%20Shop%20List MasterShopList))
  (bind _output_get_2 (Variables|Default|SetMaster%20Additional%20Categories AdditionalCategories))
  (Utilities|IsValid _as_shop_import_spawn :!label _label
    (:Is%20Valid
      (Default|InitializeVars _as_shop_import_spawn _output_get _output_get_2))
    (:Is%20Not%20Valid
      (Utilities|FlowControl|Delay 0.5)
      (goto _label))))

(event EventSend/ReceiveInstanceRef
  (params (Ref :type BP%20Radius%20Game%20Instance%20Mod%20Director%20Object%20Reference))
  ;[1 1 1] Sent from the Game instance shortly after this BP is spawned or created. Sets a reference to the Mod director Game instance, mainly for access to the Mod data actor array and the contents within.
  (|CallParentFunction Ref))

(event EventModDirectorLoadFinished
  (params (Finished :type Boolean))
  ;[1 1 1] Called by the game instance after all Mod data actors have spawned.
  (|CallParentFunction Finished))

(event EventInGameMenuOpened
  ;[1 1 1] Called any time the ingame menu is opened or closed.
)

(event EventOnIngameMenuClosed
  ;[1 1 1] Called any time the ingame menu is opened or closed.
)

(event EventOnFinishLevelLoad
  (params (Level%20Tag :type Gameplay%20Tag%20Structure))
  ;[1 1 1] Never called as this actor is killed and respawned on level change. Use the BP_MDObject if you want a persistent object that will not despawn and will call this node
)

(fn ConstructionScript)

(fn SpawnIteminBin
  (params (SoftClassPath :type Soft%20Class%20Path%20Structure))
  (bind _returnvalue (Class|KismetSystemLibrary|ToSoftClassRef(SoftClassPath) SoftClassPath))
  (CallFunction|PrinttoModLoader (Utilities|ToString(SoftClassReference) _returnvalue))
  (bind _returnvalue_2 (Utilities|LoadClassAssetBlocking _returnvalue))
  (bind _asactor (Utilities|Casting|CastToActorClass _returnvalue_2)
    (:then
      (bind _returnvalue_3 (Game|SpawnActorfromClass _asactor (Variables|Default|GetSpawnTransform) "AlwaysSpawn" "OverrideRootScale" 0 0))
      (Utilities|IsValid _returnvalue_3
        (:Is%20Valid
          (bind _asradius_item_base (Utilities|Casting|CastToRadiusItemBase _returnvalue_3))
          (bind _output_get (Variables|Default|SetSpawned%20Item _asradius_item_base))
          (Utilities|Struct|SetmembersinItemConfiguration (Variables|/Script/IntoTheRadius2.RadiusItemBase|GetItemConfiguration _output_get) true)
          (CallFunction|RotateDoorandWait)
          (return true))
        (:Is%20Not%20Valid
          (return false))))
    (:CastFailed
      (CallFunction|PrinttoModLoader "Cast to actor class failed"))))