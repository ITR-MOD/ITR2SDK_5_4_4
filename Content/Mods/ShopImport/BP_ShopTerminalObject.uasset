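; Mod director object that builds a combined shop catalogue from installed mods and supplies it to the shop terminal in the Hub level.
; When the mod director finishes loading, it gathers data assets from mod data actors marked with a magic SpecialInteger.
; Their PDA_ShopItems item and category maps merge into master maps.
; On Hub load, it spawns or reuses a BP_ShopTerminalActor and sends it both maps.
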(event Custom|CustomEvent
  (params (Message :type String))
  ;[1 0 0] DO NOT TOUCH - UE4SS Functions
)

(event EventModDirectorLoadFinished
  (params (Finished :type Boolean))
  (|CallParentFunction Finished)
  (for _array_element (Variables|/Game/ITR2/BPs/Game/BP_RadiusGameInstance_ModDirector.BP_RadiusGameInstance_ModDirector_C|GetMod%20Data%20Actor%20Array (Variables|Default|GetMod%20Director%20Ref))
    (if (== (Variables|/Game/Mods/ModDirector/ModDataActor.ModDataActor_C|GetSpecial%20Integer _array_element) 99886688)
      (Utilities|Array|AppendArray (Variables|Default|GetDA%20Array) (Variables|/Game/Mods/ModDirector/ModDataActor.ModDataActor_C|GetDA_Array _array_element))))
  (for _array_element_2 (Variables|Default|GetDA%20Array)
    (bind _aspda_shop_items (Utilities|Casting|CastToPDA_ShopItems _array_element_2))
    (bind _output_get (Variables|Default|SetCurrent%20DA _aspda_shop_items))
    (Utilities|FlowControl|Sequence
      (:then_0
        (bind _keys (Utilities|Map|Keys (Variables|/Game/Mods/ShopImport/Data/PDA_ShopItems.PDA_ShopItems_C|GetShopItemList _output_get)))
        (for _array_element_3 _keys
          (Utilities|Map|Add (Variables|Default|GetShop%20Item%20List%20Master) _array_element_3 (.Value (Utilities|Map|Find (Variables|/Game/Mods/ShopImport/Data/PDA_ShopItems.PDA_ShopItems_C|GetShopItemList _output_get) _array_element_3)))))
      (:then_1
        (bind _keys_2 (Utilities|Map|Keys (Variables|/Game/Mods/ShopImport/Data/PDA_ShopItems.PDA_ShopItems_C|GetAdditionalCategories _output_get)))
        (for _array_element_4 _keys_2
          (Utilities|Map|Add (Variables|Default|GetAdditional%20Categories%20Master) _array_element_4 (.Value (Utilities|Map|Find (Variables|/Game/Mods/ShopImport/Data/PDA_ShopItems.PDA_ShopItems_C|GetAdditionalCategories _output_get) _array_element_4))))))))

(event EventSend/ReceiveInstanceRef
  (params (Ref :type BP%20Radius%20Game%20Instance%20Mod%20Director%20Object%20Reference))
  ;[1 1 1] Called by the game instance as your BP_MDObject is Constructed.
  (|CallParentFunction Ref))

(event EventOnIngameMenuClosed
  ;[1 1 1] Called any time the ingame menu is opened or closed.
)

(event EventInGameMenuOpened
  ;[1 1 1] Called any time the ingame menu is opened or closed.
)

(event EventOnFinishLevelLoad
  (params (Level%20Tag :type Gameplay%20Tag%20Structure))
  (bind _mod_director_ref (Variables|Default|GetMod%20Director%20Ref))
  (if (== Level%20Tag "(TagName=\"Level.Hub\")")
    (bind _outactors (Default|GenericGetAllActorsOfClass _mod_director_ref "/Game/Mods/ShopImport/BP_ShopTerminalActor.BP_ShopTerminalActor_C"))
    (if (Utilities|Array|IsEmpty _outactors)
      (bind _returnvalue (Default|GenericSpawnActor _mod_director_ref "/Game/Mods/ShopImport/BP_ShopTerminalActor.BP_ShopTerminalActor_C" (Math|Transform|MakeTransform (Variables|Default|GetSpawn%20Transform%20Location) "0.000000,180.000000,0.000000" "1.000000,1.000000,1.000000") "AlwaysSpawn"))
      (bind _asbp_shop_terminal_actor (Utilities|Casting|CastToBP_ShopTerminalActor _returnvalue))
      (bind _output_get (Variables|Default|SetAs%20BP%20Shop%20Terminal%20Actor _asbp_shop_terminal_actor))
      (Class|BPIShopTerminal|SendMasterShopList(Message) _output_get (Variables|Default|GetShop%20Item%20List%20Master) (Variables|Default|GetAdditional%20Categories%20Master))
      (else
        (bind _asbp_shop_terminal_actor_2 (Utilities|Casting|CastToBP_ShopTerminalActor (Utilities|Array|Get(acopy) _outactors)))
        (bind _output_get_2 (Variables|Default|SetAs%20BP%20Shop%20Terminal%20Actor _asbp_shop_terminal_actor_2))
        (Class|BPIShopTerminal|SendMasterShopList(Message) _output_get_2 (Variables|Default|GetShop%20Item%20List%20Master) (Variables|Default|GetAdditional%20Categories%20Master))))))