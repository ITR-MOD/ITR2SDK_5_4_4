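; BP_MDObject_Example is a sample Mod Director object that shows the event hooks available to a mod.
; It prints the gameplay tag of each loaded level to the mod loader and leaves the in-game menu and UE4SS events empty.
; When Mod Director finishes loading, it scans the director's mod data actors for a magic SpecialInteger and merges their actor and object arrays into its own.
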(event Custom|CustomEvent
  (params (Message :type String))
  ;[1 0 0] DO NOT TOUCH - UE4SS Functions
)

(event EventModDirectorLoadFinished
  (params (Finished :type Boolean))
  ;[1 1 1] Sent from the Game instance shortly after this BP is spawned or created. Sets a reference to the Mod director Game instance, mainly for access to the Mod data actor array and the contents within.
  (|CallParentFunction Finished)
  (Variables|Default|SetTemp%20Actor%20Array (Variables|Default|GetMy%20Actor%20Array))
  (Variables|Default|SetTemp%20Object%20Array (Variables|Default|GetMy%20Object%20Array))
  (for _array_element (Variables|/Game/ITR2/BPs/Game/BP_RadiusGameInstance_ModDirector.BP_RadiusGameInstance_ModDirector_C|GetMod%20Data%20Actor%20Array (Variables|Default|GetMod%20Director%20Ref))
    (if (== (Variables|/Game/Mods/ModDirector/ModDataActor.ModDataActor_C|GetSpecial%20Integer _array_element) 777)
      (Utilities|Array|AppendArray (Variables|Default|GetTemp%20Actor%20Array) (Variables|/Game/Mods/ModDirector/ModDataActor.ModDataActor_C|GetOtherActorArray _array_element))
      (Utilities|Array|AppendArray (Variables|Default|GetTemp%20Object%20Array) (Variables|/Game/Mods/ModDirector/ModDataActor.ModDataActor_C|GetOtherObjectArray _array_element))))
  (Variables|Default|SetMy%20Actor%20Array (Variables|Default|GetTemp%20Actor%20Array))
  (Variables|Default|SetMy%20Object%20Array (Variables|Default|GetTemp%20Object%20Array)))

(event EventSend/ReceiveInstanceRef
  (params (Ref :type BP%20Radius%20Game%20Instance%20Mod%20Director%20Object%20Reference))
  ;[1 1 1] Called by the game instance as your BP_MDObject is Constructed.
  (|CallParentFunction Ref))

(event EventOnIngameMenuClosed
  ;[1 1 1] Called any time the ingame menu is opened or closed.
)

(event EventInGameMenuOpened
  ;[1 1 1] Called any time the ingame menu is opened or closed.
)

(event EventOnFinishLevelLoad
  (params (Level%20Tag :type Gameplay%20Tag%20Structure))
  ;[1 1 1] Called every time a level finishes loading, is sent the gameplay tag for the newly loaded level.
  (CallFunction|PrinttoModLoader (Utilities|String|Append "Mod Object Example Telling you this level tag is: " (GameplayTags|GetDebugStringfromGameplayTag Level%20Tag))))