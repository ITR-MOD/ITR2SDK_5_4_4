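; BP_RadiusGameInstance is the game instance Blueprint, holding hooks for session invites and game start.
; A received invite is logged and stored as InviteSessionToJoin with an InviteReceived flag.
; Game start binds to the main-menu-loaded event of RadiusEventsSubsystem, but that handler is empty.
; CheckInviteAndJoin only binds a success delegate; the JoinRadiusGame calls never run, and SaveConfigReport is an empty stub.
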(event Custom|CheckInviteAndJoin
  (EventDispatchers|BindEventtoOnSuccess (EventDispatchers|CreateEvent :!event Custom|OnSuccess_89CB94F44AA6E1B07EE677A284C6F0EF)))

(event Custom|OnMainMenuLoaded_Event)

(event Custom|OnFailure_89CB94F44AA6E1B07EE677A284C6F0EF)

(event Custom|OnSuccess_89CB94F44AA6E1B07EE677A284C6F0EF)

(event EventOnSessionInviteReceived
  (params (LocalPlayerNum :type Integer) (PersonInviting :type BP%20Unique%20Net%20Id%20Structure) (AppId :type String) (SessionToJoin :type Blueprint%20Session%20Result%20Structure%20%28by%20ref%29))
  (Class|FLHelpers|RadiusLog "BP_RadiusGameInstance::OnSessionInviteAccepted" "Message")
  (Variables|Default|SetbInviteReceived true)
  (Variables|Default|SetInviteSessionToJoin SessionToJoin))

(event EventOnGameStart
  (EventDispatchers|BindEventtoOnMainMenuLoaded (Subsystems|GetRadiusEventsSubsystem) (delegate Custom|OnMainMenuLoaded_Event)))

(fn SaveConfigReport)