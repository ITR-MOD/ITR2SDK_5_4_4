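; Modded Radius game instance that acts as a mod director, loading mods and relaying game events to them.
; After game start and load, it scans for ModDataActors and legacy ModActor_C actors, then spawns their listed actors and constructs their objects.
; It passes itself to new mod instances and forwards load and menu events, though menu close sends constructed objects the opened message.
; Each level load respawns the stored actor classes.
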(event Custom|PrintToModLoader
  (params (Message :type String)))

(event Custom|On%20Game%20Start%20Event)

(event Custom|On%20Finish%20Level%20Load%20Event
  (bind _asradius_player_character (Utilities|Casting|CastToRadiusPlayerCharacter (Game|GetPlayerCharacter 0))
    (:then
      (bind _output_get (Variables|Default|SetAs%20Radius%20Player%20Character _asradius_player_character))
      (Utilities|IsValid _output_get
        (:Is%20Valid
          (CallFunction|PrinttoModLoader "Got Player Character 0"))
        (:Is%20Not%20Valid
          (CallFunction|PrinttoModLoader "Cast to Radius Player Character Failed" :!label _label))))
    (:CastFailed
      (goto _label)))
  (CallFunction|PrinttoModLoader "Modded Instance on finish level load")
  (for _array_element (Variables|Default|GetConstructed%20Object%20Array)
    (Class|BPIModDirector|OnFinishLevelLoad(Message) _array_element (Class|RadiusLevelSubsystem|GetCurrentLevel (Subsystems|GetRadiusLevelSubsystem))))
  (CallFunction|RespawnActors (Variables|Default|GetLoaded%20Actors))
  (CallFunction|RespawnActors (Variables|Default|GetLegacyModActors)))

(event Custom|InGameMenuOpened%20Event
  (for _array_element (Variables|Default|GetSpawned%20Actor%20Array)
    (Class|BPIModDirector|InGameMenuOpened(Message) _array_element))
  (for _array_element_2 (Variables|Default|GetConstructed%20Object%20Array)
    (Class|BPIModDirector|InGameMenuOpened(Message) _array_element_2)))

(event Custom|OnIngameMenuClosed%20Event
  (for _array_element (Variables|Default|GetSpawned%20Actor%20Array)
    (Class|BPIModDirector|OnIngameMenuClosed(Message) _array_element))
  (for _array_element_2 (Variables|Default|GetConstructed%20Object%20Array)
    (Class|BPIModDirector|InGameMenuOpened(Message) _array_element_2)))

(event EventOnGameStart
  (bind _returnvalue (Subsystems|GetRadiusEventsSubsystem))
  (|CallParentFunction)
  (EventDispatchers|BindEventtoOnGameStart _returnvalue (delegate Custom|On%20Game%20Start%20Event))
  (EventDispatchers|BindEventtoOnFinishLoadLevel _returnvalue (delegate Custom|On%20Finish%20Level%20Load%20Event))
  (EventDispatchers|BindEventtoOnIngameMenuOpened _returnvalue (delegate Custom|InGameMenuOpened%20Event))
  (EventDispatchers|BindEventtoOnIngameMenuClosed _returnvalue (delegate Custom|OnIngameMenuClosed%20Event))
  (CallFunction|PrinttoModLoader "Modded Instance initialized, delaying for MDactors to spawn")
  (if (Class|RadiusGameInstanceInterface|IsLoadLevelFinished) :!label _label
    (CallFunction|PrinttoModLoader "Modded Instance: Game Finished loading, delaying for Mod Data actors to spawn")
    (Utilities|FlowControl|Delay 0.5)
    (CallFunction|ScanandSpawn)
    (else
      (Utilities|FlowControl|Delay 0.2)
      (goto _label))))

(event EventInit
  (|CallParentFunction))

(fn RespawnActors
  (params (Actor%20Input :type Array%20of%20Actor%20Class%20References))
  (for _array_element Actor%20Input
    (CallFunction|PrinttoModLoader (Utilities|String|Append "" "Respawning " (Utilities|GetClassDisplayName _array_element)))
    (Game|SpawnActorfromClass _array_element (Math|Transform|MakeTransform "0, 0, 0" "0, 0, 0" "1.000000,1.000000,1.000000") "AlwaysSpawn" "SelectDefaultAtRuntime" 0 0)))

(fn ScanandSpawn
  (CallFunction|PrinttoModLoader "Modded instance beginning scan for mod actors")
  (bind _outactors (Actor|GetAllActorsOfClass "/Script/Engine.Actor"))
  (for _array_element _outactors
    (bind _asmod_data_actor (Utilities|Casting|CastToModDataActor _array_element)
      (:then
        (bind _output_get (Variables|Default|SetCurrent%20Mod%20Data%20Actor _asmod_data_actor))
        (Utilities|Array|Add (Variables|Default|GetMod%20Data%20Actor%20Array) _output_get)
        (CallFunction|PrinttoModLoader (Utilities|String|Append "Found " (Variables|/Game/Mods/ModDirector/ModDataActor.ModDataActor_C|GetModName _output_get) " Version " (Utilities|String|ToString(Integer) (Variables|/Game/Mods/ModDirector/ModDataActor.ModDataActor_C|GetModVersion _output_get))))
        (CallFunction|PrinttoModLoader (Utilities|String|Append "By" (Variables|/Game/Mods/ModDirector/ModDataActor.ModDataActor_C|GetModAuthor _output_get)))
        (for _array_element_2 (Variables|/Game/Mods/ModDirector/ModDataActor.ModDataActor_C|GetModActorArray _output_get)
          (Utilities|Array|AddUnique (Variables|Default|GetLoaded%20Actors) _array_element_2))
        (for _array_element_3 (Variables|/Game/Mods/ModDirector/ModDataActor.ModDataActor_C|GetModObjectArray _output_get)
          (Utilities|Array|AddUnique (Variables|Default|GetLoaded%20Objects) _array_element_3)))
      (:CastFailed
        (CallFunction|PrinttoModLoader (.RightS (Utilities|String|Split (Utilities|BreakSoftObjectPath (Class|KismetSystemLibrary|GetSoftClassPath (Utilities|GetClass _array_element))) "." "IgnoreCase" "FromEnd")))
        (if (Utilities|Enum|Equal(Enum) (.RightS (Utilities|String|Split (Utilities|BreakSoftObjectPath (Class|KismetSystemLibrary|GetSoftClassPath (Utilities|GetClass _array_element))) "." "IgnoreCase" "FromEnd")) "ModActor_C")
          (Utilities|Array|Add (Variables|Default|GetLegacyModActors) (Utilities|GetClass _array_element))))))
  (CallFunction|Spawn (Variables|Default|GetLoaded%20Actors))
  (CallFunction|Spawn (Variables|Default|GetLegacyModActors))
  (for _array_element_4 (Variables|Default|GetLoaded%20Objects)
    (bind _output_get_2 (Variables|Default|SetCurrent%20Object _array_element_4))
    (bind _returnvalue (Game|ConstructObjectfromClass _output_get_2))
    (CallFunction|PrinttoModLoader (Utilities|String|Append "Constructing " (Utilities|GetClassDisplayName _output_get_2)))
    (Class|BPIModDirector|Send/ReceiveInstanceRef(Message) _returnvalue self)
    (Utilities|Array|Add (Variables|Default|GetConstructed%20Object%20Array) _returnvalue))
  (for _array_element_5 (Variables|Default|GetSpawned%20Actor%20Array)
    (Class|BPIModDirector|ModDirectorLoadFinished(Message) _array_element_5 true))
  (for _array_element_6 (Variables|Default|GetConstructed%20Object%20Array)
    (Class|BPIModDirector|ModDirectorLoadFinished(Message) _array_element_6 true))
  (CallFunction|PrinttoModLoader "Scan and Spawn Function complete"))

(fn Spawn
  (params (Array :type Array%20of%20Actor%20Class%20References))
  (for _array_element Array
    (bind _output_get (Variables|Default|SetCurrentModActor _array_element))
    (bind _outactors (Actor|GetAllActorsOfClass _output_get))
    (if (!= (Utilities|Array|Length _outactors) 0)
      (CallFunction|PrinttoModLoader (Utilities|String|Append (Utilities|GetClassDisplayName _output_get) " is already spawned!"))
      (elif (Utilities|IsValidClass _output_get)
        (CallFunction|PrinttoModLoader (Utilities|String|Append (Utilities|GetClassDisplayName _output_get) " Is Valid"))
        (bind _returnvalue (Game|SpawnActorfromClass (Variables|Default|GetCurrentModActor) (Math|Transform|MakeTransform "0, 0, 0" "0, 0, 0" "1.000000,1.000000,1.000000") "AlwaysSpawn" "SelectDefaultAtRuntime" 0 0))
        (bind _asbp_mdactor (Utilities|Casting|CastToBP_MDActor _returnvalue)
          (:then
            (Class|BPIModDirector|Send/ReceiveInstanceRef(Message) _asbp_mdactor self)
            (Utilities|Array|Add (Variables|Default|GetSpawned%20Actor%20Array) _asbp_mdactor))
          (:CastFailed
            (Utilities|Time|SetTimerbyFunctionName _returnvalue "PostBeginPlay" 0.0)
            (Utilities|Array|Add (Variables|Default|GetSpawnedLegacyActorArray) _returnvalue)))
        (else
          (CallFunction|PrinttoModLoader (Utilities|String|Append (Utilities|GetClassDisplayName _output_get) " not a valid class")))))))

(fn GenericSpawnActor
  (params (Actor :type Actor%20Class%20Reference) (SpawnTransform :type Transform) (CollisionHandlingOverride :type ESpawnActorCollisionHandlingMethod%20Enum :default "Undefined") (Instigator :type Pawn%20Object%20Reference))
  (bind _returnvalue (Game|SpawnActorfromClass Actor SpawnTransform CollisionHandlingOverride "MultiplyWithRoot" 0 Instigator))
  (return _returnvalue))

(fn GenericGetAllActorsOfClass
  (params (ActorClass :type Actor%20Class%20Reference))
  (bind _outactors (Actor|GetAllActorsOfClass ActorClass))
  (return _outactors))

(fn GenericGetOneActorOfClass
  (params (ActorClass :type Actor%20Class%20Reference))
  (bind _returnvalue (Actor|GetActorOfClass ActorClass))
  (return _returnvalue))